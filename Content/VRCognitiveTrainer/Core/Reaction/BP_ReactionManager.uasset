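; Manager actor for the VR cognitive trainer's reaction exercise, spawning and tracking interactable BP_Target actors.
; CreateTargets clears existing targets, then spawns new ones at random points inside a box defined by two corner offsets from the actor's location.
; Each target's OnInteracted is bound to an event, and EventTargetHit moves a hit target to a new random point instead of respawning it, then broadcasts OnTargetHit.
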(event Custom|EventTargetHit
  (params (Target :type BP%20Target%20Object%20Reference))
  (bind _location (CallFunction|GenerateLocation))
  (Transformation|SetActorLocation Target _location false false)
  (Default|CallOnTargetHit))

(event Custom|CreateTargets
  (CallFunction|ClearTargets)
  (for _index (range 0 (Variables|Config|GetTargetNum))
    (bind _location (CallFunction|GenerateLocation))
    (bind _returnvalue (Game|SpawnActorfromClass "/Game/VRCognitiveTrainer/Core/Reaction/BP_Target.BP_Target_C" (Math|Transform|MakeTransform _location "0, 0, 0" "1.000000,1.000000,1.000000") "AdjustIfPossibleButAlwaysSpawn" "MultiplyWithRoot" 0 0))
    (EventDispatchers|BindEventtoOnInteracted _returnvalue (EventDispatchers|CreateEvent :!event Custom|EventTargetHit))
    (Utilities|Array|Add (Variables|Default|GetTargets) _returnvalue)))

(event Custom|ClearTargets
  (for _array_element (Variables|Default|GetTargets)
    (Actor|DestroyActor _array_element))
  (Utilities|Array|Clear (Variables|Default|GetTargets)))

(event EventBeginPlay)

(fn ConstructionScript)

(fn GenerateLocation
  (bind _returnvalue (Transformation|GetActorLocation))
  (bind _returnvalue_2 (Transformation|GetActorLocation))
  (bind _boxpointa (Variables|Config|GetBoxPointA))
  (bind _boxpointb (Variables|Config|GetBoxPointB))
  (bind _returnvalue_3 (+ _returnvalue _boxpointb))
  (bind _returnvalue_4 (+ _returnvalue_2 _boxpointa))
  (bind (_x _y _z) (Math|Vector|BreakVector _returnvalue_4))
  (bind (_x_2 _y_2 _z_2) (Math|Vector|BreakVector _returnvalue_3))
  (return (Math|Vector|MakeVector (Math|Random|RandomFloatinRange (Math|Float|Min(Float) _x _x_2) (Math|Float|Max(Float) _x _x_2)) (Math|Random|RandomFloatinRange (Math|Float|Min(Float) _y _y_2) (Math|Float|Max(Float) _y _y_2)) (Math|Random|RandomFloatinRange (Math|Float|Min(Float) _z _z_2) (Math|Float|Max(Float) _z _z_2)))))