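; Game mode for the Reaction exercise in VRCognitiveTrainer, running a timed round in which target hits earn points.
; On BeginPlay it finds the level's BP_ReactionManager and binds to its target-hit event.
; Game start sets the round timer, has the manager create targets and resets the score, while game finish clears the targets.
; Each hit adds ScorePerObject and broadcasts the new score through OnScoreUpdated.
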(event Custom|OnTimerFinished
  (CallFunction|GameFinished))

(event Custom|OnTargetHit
  (bind _output_get (Variables|Default|SetScore (+ (Variables|Default|GetScore) (Variables|Default|GetScorePerObject))))
  (Default|CallOnScoreUpdated _output_get))

(event EventBeginPlay
  (|CallParentFunction)
  (bind _outactors (Actor|GetAllActorsOfClass "/Game/VRCognitiveTrainer/Core/Reaction/BP_ReactionManager.BP_ReactionManager_C"))
  (bind _output_get (Variables|Default|SetManager (Utilities|Array|Get(acopy) _outactors)))
  (EventDispatchers|BindEventtoOnTargetHit _output_get (EventDispatchers|CreateEvent :!event Custom|OnTargetHit)))

(event EventGameFinished
  (|CallParentFunction)
  (Default|ClearTargets (Variables|Default|GetManager)))

(event EventGameStarted
  (|CallParentFunction)
  (bind _returnvalue (Utilities|Time|SetTimerbyEvent (EventDispatchers|CreateEvent :!event Custom|OnTimerFinished) (Variables|Default|GetTime) false false 1.0))
  (Variables|Default|SetTimer _returnvalue)
  (Default|CreateTargets (Variables|Default|GetManager))
  (Variables|Default|SetScore 0)
  (Default|CallOnScoreUpdated (Variables|Default|GetScore)))

(fn ConstructionScript
  (|CallParentFunction))