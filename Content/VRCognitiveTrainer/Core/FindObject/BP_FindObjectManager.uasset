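; BP_FindObjectManager runs the find-object task in the VR cognitive trainer, choosing which registered object is the current target.
; Object components register into a list, and the manager binds to each one's interaction event.
; GenerateObjectToFind clears all target flags, then rerolls a random pick until it differs from the previous one, looping endlessly if no different index exists.
; The target interaction handler fires the OnObjectFound dispatcher.
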(event Custom|OnTargetObjectInteracted
  (params (Component :type BPC%20Object%20to%20Find%20Object%20Reference))
  (Default|CallOnObjectFound))

(event Custom|GenerateObjectToFind
  (CallFunction|ClearObjects)
  (bind _output_get (Variables|Default|SetSelectedObjectIndex (.OutIndex (Utilities|Array|Random (Variables|Default|GetObjectComponents))) :!label _label))
  (if (!= _output_get (Variables|Default|GetLastSelectedObjectIndex))
    (bind _output_get_2 (Variables|Default|SetSelectedTarget (Utilities|Array|Get(acopy) (Variables|Default|GetObjectComponents) (Variables|Default|GetSelectedObjectIndex))))
    (Default|SetTarget _output_get_2 true)
    (Variables|Default|SetLastSelectedObjectIndex (Variables|Default|GetSelectedObjectIndex))
    (else
      (goto _label))))

(event Custom|ClearObjects
  (Variables|Default|SetSelectedTarget 0)
  (for _array_element (Variables|Default|GetObjectComponents)
    (Default|SetTarget _array_element false)))

(event EventBeginPlay)

(fn ConstructionScript)

(fn RegisterComponent
  (params (Object :type BPC%20Object%20to%20Find%20Object%20Reference))
  (Utilities|Array|AddUnique (Variables|Default|GetObjectComponents) Object)
  (EventDispatchers|BindEventtoOnInteracted Object (EventDispatchers|CreateEvent :!event Custom|OnTargetObjectInteracted)))

(fn UnregisterComponent
  (params (Item :type BPC%20Object%20to%20Find%20Object%20Reference%20%28by%20ref%29))
  (Utilities|Array|RemoveItem (Variables|Default|GetObjectComponents) Item))