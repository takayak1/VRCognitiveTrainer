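; Game mode for the find-object minigame in the VR cognitive trainer, running a timed, scored round.
; On start it arms a timer, resets the score, asks BP_FindObjectManager for an object and moves the player to a target location.
; Each found-object event from the manager adds points and generates the next object.
; Finishing clears the objects and returns the player to the saved location.
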(event Custom|OnObjectFound
  (bind _output_get (Variables|Default|SetScore (+ (Variables|Default|GetScore) (Variables|Default|GetScorePerObject))))
  (Default|CallOnScoreUpdated _output_get)
  (Default|GenerateObjecttoFind (Variables|Default|GetManager)))

(event Custom|OnTimerFinished
  (CallFunction|GameFinished))

(event EventBeginPlay
  (bind _outactors (Actor|GetAllActorsOfClass "/Game/VRCognitiveTrainer/Core/FindObject/BP_FindObjectManager.BP_FindObjectManager_C"))
  (Variables|Default|SetManager (Utilities|Array|Get(acopy) _outactors))
  (EventDispatchers|BindEventtoOnObjectFound (Variables|Default|GetManager) (EventDispatchers|CreateEvent :!event Custom|OnObjectFound)))

(event EventGameFinished
  (|CallParentFunction)
  (Default|ClearObjects (Variables|Default|GetManager))
  (Transformation|SetActorLocation (Game|Player|GetPlayerPawn 0) (Variables|Default|GetPlayerLocation) false false))

(event EventGameStarted
  (|CallParentFunction)
  (bind _returnvalue (Utilities|Time|SetTimerbyEvent (EventDispatchers|CreateEvent :!event Custom|OnTimerFinished) (Variables|Default|GetTime) false false 1.0))
  (Variables|Default|SetTimer _returnvalue)
  (Default|GenerateObjecttoFind (Variables|Default|GetManager))
  (Variables|Default|SetScore 0)
  (Default|CallOnScoreUpdated (Variables|Default|GetScore))
  (Variables|Default|SetPlayerLocation (Transformation|GetActorLocation (Game|Player|GetPlayerPawn 0)))
  (Transformation|SetActorLocation (Game|Player|GetPlayerPawn 0) (Transformation|GetActorLocation (Variables|Config|GetTargetLocation)) false false))

(fn ConstructionScript)