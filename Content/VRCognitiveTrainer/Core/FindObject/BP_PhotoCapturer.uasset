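; BP_PhotoCapturer takes a snapshot of a given actor, apparently for the FindObject part of the VR cognitive trainer.
; Its Capture event saves the actor's location and rotation, then moves it to the Scene component's world transform.
; It triggers the SceneCaptureComponent2D and puts the actor back immediately, all without delay.
; The Delay nodes in the graph are disconnected and never run.
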(event Custom|Capture
  (params (TargetActor :type Actor%20Object%20Reference))
  (bind _scene (Variables|Default|GetScene))
  (Variables|Default|SetTargetActorInitialLocation (Transformation|GetActorLocation TargetActor))
  (Variables|Default|SetTargetActorInitialRotation (Transformation|GetActorRotation TargetActor))
  (Transformation|SetActorLocationAndRotation TargetActor (Transformation|GetWorldLocation _scene) (Transformation|GetWorldRotation _scene))
  (Rendering|SceneCapture|CaptureScene (Variables|Default|GetSceneCaptureComponent2D) :!class /Script/Engine.SceneCaptureComponent2D)
  (Transformation|SetActorLocationAndRotation TargetActor (Variables|Default|GetTargetActorInitialLocation) (Variables|Default|GetTargetActorInitialRotation)))

(event EventBeginPlay)

(event Collision|EventActorBeginOverlap
  (params (OtherActor :type Actor%20Object%20Reference)))

(event EventTick
  (params (DeltaSeconds :type Float%20%28single-precision%29)))

(fn ConstructionScript)