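; BPC_ObjectToFind is an actor component that makes its owner a findable object in the VR cognitive trainer's find-object task.
; It registers with BP_FindObjectManager on BeginPlay and unregisters on EndPlay.
; SetTarget toggles the target flag and swaps the owner's mesh material.
; Actor hits or Interact calls trigger interaction, which broadcasts OnInteracted and plays right-hand haptics only when it is the target.
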(event Custom|OnParentHit
  (params (SelfActor :type Actor%20Object%20Reference) (OtherActor :type Actor%20Object%20Reference) (NormalImpulse :type Vector) (Hit :type Hit%20Result%20Structure%20%28by%20ref%29))
  (CallFunction|HandleInteraction))

(event Custom|SetTarget
  (params (bTarget :type Boolean))
  (Variables|Default|SetTarget bTarget)
  (Rendering|Material|SetMaterial (Actor|GetComponentbyClass (Components|GetOwner) "/Script/Engine.StaticMeshComponent") 0 (select (Variables|Default|GetTarget) "/Game/VRCognitiveTrainer/Core/Materials/MI_Grid_Target.MI_Grid_Target" "/Game/VRCognitiveTrainer/Core/Materials/MI_Grid_Default.MI_Grid_Default")))

(event Custom|RegisterComponent
  (bind _outactors (Actor|GetAllActorsOfClass "/Game/VRCognitiveTrainer/Core/FindObject/BP_FindObjectManager.BP_FindObjectManager_C"))
  (Variables|Default|SetManager (Utilities|Array|Get(acopy) _outactors))
  (Default|RegisterComponent (Variables|Default|GetManager) self))

(event Custom|HandleInteraction
  (Development|PrintText "Interacted")
  (if (Variables|Default|GetTarget)
    (Default|CallOnInteracted self)
    (Class|PlayerController|PlayHapticEffect (Game|GetPlayerController 0) "/Game/VRTemplate/Haptics/GrabHapticEffect.GrabHapticEffect" "Right" 1.0 false)))

(event EventBeginPlay
  (|CallParentFunction)
  (CallFunction|RegisterComponent)
  (Collision|BindEventtoOnActorHit (Components|GetOwner) (EventDispatchers|CreateEvent :!event Custom|OnParentHit)))

(event EventEndPlay
  (params (EndPlayReason :type EEndPlayReason%20Enum :default "Destroyed"))
  (Default|UnregisterComponent (Variables|Default|GetManager) self))

(event EventInteract
  (CallFunction|HandleInteraction))