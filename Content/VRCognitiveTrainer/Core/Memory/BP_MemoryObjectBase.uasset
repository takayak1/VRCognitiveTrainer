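; BP_MemoryObjectBase is the base actor for interactable objects in the VR cognitive trainer's memory module.
; Interact broadcasts OnInteracted with itself, then plays a timeline that drives a uniform actor scale offset from 1.0 as visual feedback.
; SetIndex stores the object's index and displays it on a TextRender component.
; Initialize takes a config but is empty here, as is the construction script.
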(event Custom|SetIndex
  (params (Index :type Integer))
  (bind _output_get (Variables|Default|SetIndex Index))
  (Rendering|Components|TextRender|SetText (Variables|Default|GetTextRender) (Utilities|Text|ToText(Integer) _output_get)))

(event Custom|Initialize
  (params (Config :type BPS%20Memory%20Object%20Config%20Structure)))

(event EventInteract
  (Default|CallOnInteracted self)
  (bind _newtrack_0 (Timeline|Timeline Play)
    (:Update
      (Transformation|SetActorScale3D (Math|Vector|MakeVector (+ (* _newtrack_0 0.1) 1.0) (+ (* _newtrack_0 0.1) 1.0) (+ (* _newtrack_0 0.1) 1.0))))))

(fn ConstructionScript)