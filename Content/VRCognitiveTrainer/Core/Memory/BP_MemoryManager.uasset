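; Manager for the VR cognitive trainer's memory test, which spawns a random set of items and a shuffled answer set.
; Generate picks variant indexes from the config, optionally without duplicates by re-rolling, and places actors at manual attachments or padded offsets.
; CreateAnswerObjects spawns the shuffled copies.
; Answer interactions record actor indexes, which CheckAnswer compares in order to the generated indexes once enough are selected, then OnAnswered broadcasts the result.
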(event Custom|OnObjectInteracted
  (params (Object :type Actor%20Object%20Reference))
  (if (Utilities|Array|ContainsItem (Variables|Default|GetAnswerActors) Object)
    (bind _output_get (Variables|Default|SetLastSelectedIndex (Utilities|Array|FindItem (Variables|Default|GetAnswerActors) Object)))
    (Utilities|Array|Add (Variables|Default|GetSelectedIndexes) _output_get)
    (Development|PrintString (Utilities|String|ToString(Integer) _output_get) true true "(R=1.000000,G=0.306137,B=0.932491,A=1.000000)" 12.0)
    (if (== (Utilities|Array|Length (Variables|Default|GetSelectedIndexes)) (.NumItemsToGenerate (Utilities|Struct|BreakBPS_MemoryObjectGenerationConfig (Variables|/Game/VRCognitiveTrainer/Core/Memory/BP_MemoryTestGeneratorConfig.BP_MemoryTestGeneratorConfig_C|GetConfig (Variables|Default|GetConfig)))))
      (bind _result (CallFunction|CheckAnswer))
      (Default|CallOnAnswered _result)
      (Utilities|Array|Clear (Variables|Default|GetSelectedIndexes)))))

(event Custom|HideTestActors
  (params (bHidden :type Boolean))
  (for _array_element (Variables|Default|GetTestActors)
    (Rendering|SetActorHiddenInGame _array_element bHidden)))

(event EventBeginPlay
  (|CallParentFunction))

(fn ConstructionScript)

(fn Generate
  (params (Config :type BP%20Memory%20Test%20Generator%20Config%20Object%20Reference))
  (Variables|Default|SetConfig Config)
  (CallFunction|Clear)
  (Utilities|FlowControl|Sequence
    (:then_0
      (if (not (.bAllowDuplicates (Utilities|Struct|BreakBPS_MemoryObjectGenerationConfig (Variables|/Game/VRCognitiveTrainer/Core/Memory/BP_MemoryTestGeneratorConfig.BP_MemoryTestGeneratorConfig_C|GetConfig Config))))
        (if (> (.NumItemsToGenerate (Utilities|Struct|BreakBPS_MemoryObjectGenerationConfig (Variables|/Game/VRCognitiveTrainer/Core/Memory/BP_MemoryTestGeneratorConfig.BP_MemoryTestGeneratorConfig_C|GetConfig Config))) (Utilities|Array|Length (.Variants (Utilities|Struct|BreakBPS_MemoryObjectGenerationConfig (Variables|/Game/VRCognitiveTrainer/Core/Memory/BP_MemoryTestGeneratorConfig.BP_MemoryTestGeneratorConfig_C|GetConfig Config)))))
          (Development|PrintString "ERROR: Failed to generate unique variants" true true "(R=1.000000,G=0.000000,B=0.014804,A=1.000000)" 1e+01)
          (return))))
    (:then_1
      (for _index (range 0 (- (.NumItemsToGenerate (Utilities|Struct|BreakBPS_MemoryObjectGenerationConfig (Variables|/Game/VRCognitiveTrainer/Core/Memory/BP_MemoryTestGeneratorConfig.BP_MemoryTestGeneratorConfig_C|GetConfig Config))) 1))
        (if (.bAllowDuplicates (Utilities|Struct|BreakBPS_MemoryObjectGenerationConfig (Variables|/Game/VRCognitiveTrainer/Core/Memory/BP_MemoryTestGeneratorConfig.BP_MemoryTestGeneratorConfig_C|GetConfig Config)))
          (Utilities|Array|Add (LocalVariables|GetGeneratedIndexes) (Math|Random|RandomInteger (Utilities|Array|Length (.Variants (Utilities|Struct|BreakBPS_MemoryObjectGenerationConfig (Variables|/Game/VRCognitiveTrainer/Core/Memory/BP_MemoryTestGeneratorConfig.BP_MemoryTestGeneratorConfig_C|GetConfig Config))))))
          (else
            (LocalVariables|SetGeneratedIndes (Math|Random|RandomInteger (Utilities|Array|Length (.Variants (Utilities|Struct|BreakBPS_MemoryObjectGenerationConfig (Variables|/Game/VRCognitiveTrainer/Core/Memory/BP_MemoryTestGeneratorConfig.BP_MemoryTestGeneratorConfig_C|GetConfig Config))))) :!label _label)
            (if (not (Utilities|Array|ContainsItem (LocalVariables|GetGeneratedIndexes) (LocalVariables|GetGeneratedIndes)))
              (Utilities|Array|Add (LocalVariables|GetGeneratedIndexes) (LocalVariables|GetGeneratedIndes))
              (else
                (goto _label))))))
      (Variables|Default|SetGenerated%20Indexes (LocalVariables|GetGeneratedIndexes))
      (for _array_element (LocalVariables|GetGeneratedIndexes)
        (Utilities|Array|Add (Variables|Default|GetGenerated%20Config) (Utilities|Array|Get(acopy) (.Variants (Utilities|Struct|BreakBPS_MemoryObjectGenerationConfig (Variables|/Game/VRCognitiveTrainer/Core/Memory/BP_MemoryTestGeneratorConfig.BP_MemoryTestGeneratorConfig_C|GetConfig Config))) _array_element))
        (Development|PrintText (Utilities|Text|ToText(Integer) _array_element) true true "(R=1.000000,G=0.619206,B=0.000000,A=1.000000)" 1e+01))
      (CallFunction|CreateObjects (Variables|Default|GetGenerated%20Config) (Variables|Config|GetManualAttachments) false))))

(fn CreateObjects
  (params (Objects :type Array%20of%20BPS%20Memory%20Object%20Config%20Structures) (Attachments :type Array%20of%20Actor%20Object%20References) (bAnswer :type Boolean))
  (for (_array_element _array_index) Objects
    (bind _returnvalue (Game|SpawnActorfromClass (.Class (Utilities|Struct|BreakBPS_MemoryObjectConfig _array_element)) (Math|Transform|MakeTransform "0, 0, 0" "0, 0, 0" "1.000000,1.000000,1.000000") "AlwaysSpawn" "MultiplyWithRoot" 0 0))
    (LocalVariables|SetCreatedActor _returnvalue)
    (Utilities|FlowControl|Sequence
      (:then_0
        (if (Utilities|IsValid (Utilities|Array|Get(acopy) Attachments _array_index))
          (LocalVariables|SetResultLocation (Transformation|GetActorLocation (Utilities|Array|Get(acopy) Attachments _array_index)))
          (else
            (LocalVariables|SetResultLocation (+ (Transformation|GetActorLocation (Utilities|Array|Get(acopy) Attachments (Utilities|Array|LastIndex Attachments))) (* (Variables|Config|GetPadding) _array_index))))))
      (:then_1
        (Transformation|SetActorLocation (LocalVariables|GetCreatedActor) (LocalVariables|GetResultLocation) false false))
      (:then_2
        (Utilities|Array|Add (select bAnswer (Variables|Default|GetAnswerActors) (Variables|Default|GetTestActors)) (LocalVariables|GetCreatedActor))
        (EventDispatchers|BindEventtoOnInteracted (LocalVariables|GetCreatedActor) (EventDispatchers|CreateEvent :!event Custom|OnObjectInteracted))
        (Default|Initialize (LocalVariables|GetCreatedActor) _array_element)))))

(fn CreateAnswerObjects
  (Variables|Default|SetAnswerGeneratedIndexes (Variables|Default|GetGenerated%20Indexes))
  (Utilities|Array|Shuffle (Variables|Default|GetAnswerGeneratedIndexes))
  (for _array_element (Variables|Default|GetAnswerGeneratedIndexes)
    (Utilities|Array|Add (Variables|Default|GetAnswerGeneratedObjects) (Utilities|Array|Get(acopy) (Variables|Default|GetGenerated%20Config) _array_element)))
  (CallFunction|CreateObjects (Variables|Default|GetAnswerGeneratedObjects) (Variables|Config|GetAnswerManualAttachments) true))

(fn Clear
  (Utilities|Array|Clear (Variables|Default|GetGenerated%20Config))
  (Utilities|Array|Clear (Variables|Default|GetGenerated%20Indexes))
  (Utilities|Array|Clear (Variables|Default|GetAnswerGeneratedIndexes))
  (Utilities|Array|Clear (Variables|Default|GetAnswerGeneratedObjects))
  (Utilities|FlowControl|Sequence
    (:then_0
      (for _array_element (Variables|Default|GetTestActors)
        (Actor|DestroyActor _array_element)))
    (:then_1
      (for _array_element_2 (Variables|Default|GetAnswerActors)
        (Actor|DestroyActor _array_element_2)))
    (:then_2
      (Utilities|Array|Clear (Variables|Default|GetTestActors))
      (Utilities|Array|Clear (Variables|Default|GetAnswerActors))
      (Utilities|Array|Clear (Variables|Default|GetSelectedIndexes)))))

(fn CheckAnswer
  (for (_array_element _array_index) (Variables|Default|GetGenerated%20Indexes)
    (if (not (== (Utilities|Array|Get(acopy) (Variables|Default|GetSelectedIndexes) _array_index) _array_element))
      (return false)))
  (return true))