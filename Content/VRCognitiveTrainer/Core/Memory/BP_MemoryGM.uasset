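; BP_MemoryGM is the game mode for a memory exercise in the VR cognitive trainer, running a timed memorize-then-answer round.
; On start, it has the level's BP_MemoryManager generate test actors from a random config and starts a timer.
; When time expires, the manager hides those actors and creates answer objects.
; The manager's OnAnswered event ends the round, clearing it, broadcasting the result and adding score when correct.
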(event Custom|TimerFinished
  (Default|HideTestActors (Variables|Default|GetManager) true)
  (Default|CreateAnswerObjects (Variables|Default|GetManager))
  (Default|CallOnTimerFinished)
  (Default|CallOnGenerateAnswer))

(event Custom|OnTargetHit)

(event Custom|OnAnswered
  (params (bResult :type Boolean))
  (CallFunction|GameFinished)
  (Default|CallOnResult bResult)
  (if bResult
    (bind _output_get (Variables|Default|SetScore (+ (Variables|Default|GetScore) (Variables|Default|GetScorePerObject))))
    (Default|CallOnScoreUpdated _output_get)))

(event EventBeginPlay
  (|CallParentFunction)
  (bind _outactors (Actor|GetAllActorsOfClass "/Game/VRCognitiveTrainer/Core/Memory/BP_MemoryManager.BP_MemoryManager_C"))
  (Variables|Default|SetManager (Utilities|Array|Get(acopy) _outactors))
  (EventDispatchers|BindEventtoOnAnswered (Variables|Default|GetManager) (EventDispatchers|CreateEvent :!event Custom|OnAnswered))
  (Variables|Default|SetScore 0)
  (Default|CallOnScoreUpdated (Variables|Default|GetScore)))

(event EventGameFinished
  (|CallParentFunction)
  (Default|Clear (Variables|Default|GetManager)))

(event EventGameStarted
  (|CallParentFunction)
  (bind _returnvalue (Utilities|Time|SetTimerbyEvent (EventDispatchers|CreateEvent :!event Custom|TimerFinished) (Variables|Default|GetTime) false false 1.0))
  (Variables|Default|SetTimer _returnvalue)
  (Default|Generate (Variables|Default|GetManager) (.OutItem (Utilities|Array|Random (Variables|Default|GetConfigs)))))

(fn ConstructionScript
  (|CallParentFunction))