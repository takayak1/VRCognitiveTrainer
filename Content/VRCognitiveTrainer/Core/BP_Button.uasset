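; Pressable button actor for VRCognitiveTrainer that signals when it is interacted with.
; Interact calls the OnInteracted dispatcher, then plays a sped-up Timeline that drives the relative Z of Cylinder1 to animate it.
; The Timeline uses Play rather than PlayFromStart, and a material-swap flash between accent and target grid materials is left unconnected.
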(event EventBeginPlay)

(event Collision|EventActorBeginOverlap
  (params (OtherActor :type Actor%20Object%20Reference)))

(event EventTick
  (params (DeltaSeconds :type Float%20%28single-precision%29)))

(event EventInteract
  (Default|CallOnInteracted)
  (Components|Timeline|SetPlayRate (Variables|Default|GetTimeline) 8.0)
  (bind _newtrack_0 (Timeline|Timeline Play)
    (:Update
      (Transformation|SetRelativeLocation (Variables|Default|GetCylinder1) (Math|Vector|MakeVector 0.0 0.0 (+ (* _newtrack_0 1e+01) 1e+01)) false false))))

(fn ConstructionScript)